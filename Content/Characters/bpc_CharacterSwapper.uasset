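; Player-state component that swaps the pawn a player controls for another character.
; A server event multicasts the start of a swap, storing the chosen Character on all machines and signalling StartSwap.
; A separate server swap looks up that Character's class, spawns it at the current pawn's transform, destroys the old pawn and possesses the new one.
; It then multicasts CharacterSwapped with the new pawn and Character.
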(event `self.ReceiveBeginPlay`
  (bind _asplayer_state (cast `PlayerState` (`self.GetOwner`)))
  (set `self.PlayerController` (`PlayerState.GetPlayerController` _asplayer_state)))

(event `ServerStartSwap`
  (params (Character :type "ECharacter Enum" :default "Kazooie"))
  (`self.MulticastStartSwap` Character))

(event `ServerSwapCharacter`
  (for _array_element (`self.Characters`)
    (if (`|EnumEquality` (break `/Game/Characters/s_CharacterActors` _array_element) (`self.GetCharacter`))
      (bind _returnvalue (`|SpawnActorFromClass` (`.CharacterClass_8_60CC18854BFD965C4F462BAAC5E67749` (break `/Game/Characters/s_CharacterActors` _array_element)) (`Actor.GetTransform` (`Controller.K2_GetPawn` (`self.PlayerController`))) "AlwaysSpawn" "MultiplyWithRoot" null null))
      (`Actor.K2_DestroyActor` (`Controller.K2_GetPawn` (`self.PlayerController`)))
      (`Controller.Possess` (`self.PlayerController`) _returnvalue)
      (`self.MulticastSwap` _returnvalue))))

(event `MulticastStartSwap`
  (params (Character :type "ECharacter Enum" :default "Kazooie"))
  (`self.SetCharacter` Character)
  (`self.StartSwap`))

(event `MulticastSwap`
  (params (CharacterPawn :type "Character Object Reference"))
  (`self.CharacterSwapped` CharacterPawn (`self.GetCharacter`)))