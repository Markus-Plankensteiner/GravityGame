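; IceChicken character Blueprint that adds an ice ground-pound effect on landing.
; When it lands while GroundPounding is set, it spawns a Bp_IceWave at its location, with itself as owner and instigator.
; It then calls the parent OnLanded, leaving the rest of the landing behavior to the base class.
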(event `self.OnLanded`
  (params (Hit :type "HitResult Structure (by ref)"))
  (`|ExecutionSequence`
    (:`then_0`
      (if (`self.GroundPounding`)
        (`|SpawnActorFromClass` "/Game/Characters/IceChicken/Abilities/Icewave/bp_IceWave.bp_IceWave_C" (`KismetMathLibrary.MakeTransform` (`self.K2_GetActorLocation`)) "Undefined" "MultiplyWithRoot" self self)))
    (:`then_1`
      (`parent.OnLanded` Hit))))

(fn `UserConstructionScript`
  (`parent.UserConstructionScript`))