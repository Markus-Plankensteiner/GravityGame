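; Collectible star that completes a mission in the level when something overlaps its sphere.
; The construction script finds the mission level actor and resolves this star's mission from its index.
; On first overlap it marks that mission complete and plays a replicated collect sequence, offset to the star's transform through instance data.
; When the sequence finishes, the mission manager runs a server mission selection.
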(event `self.Sphere.OnComponentBeginOverlap`
  (params (OverlappedComponent :type "PrimitiveComponent Object Reference") (OtherActor :type "Actor Object Reference") (OtherComp :type "PrimitiveComponent Object Reference") (OtherBodyIndex :type Integer) (bFromSweep :type Boolean) (SweepResult :type "HitResult Structure (by ref)"))
  (`/Engine/EditorBlueprintResources/StandardMacros.DoOnce` false
    (:`Completed`
      (`self.Create Level Sequence`))))

(event `Create Level Sequence`
  (bind _outactor (`LevelSequencePlayer.CreateLevelSequencePlayer` "/Game/Gameplay/Collectibles/Star/ls_CollectStar.ls_CollectStar" (make `MovieSceneSequencePlaybackSettings` false)))
  (`self.SetReplicates` _outactor true)
  (set `LevelSequenceActor.bReplicatePlayback` true _outactor)
  (set `LevelSequenceActor.bOverrideInstanceData` true _outactor)
  (bind _asdefault_level_sequence_instance_data (cast `DefaultLevelSequenceInstanceData` (`LevelSequenceActor.DefaultInstanceData` _outactor)))
  (set `DefaultLevelSequenceInstanceData.TransformOrigin` (`self.GetTransform`) _asdefault_level_sequence_instance_data)
  (bind _sequenceplayer (`LevelSequenceActor.SequencePlayer` _outactor))
  (add `MovieSceneSequencePlayer.OnFinished` _sequenceplayer (delegate `OnFinished`))
  (`/Game/Gameplay/Missions/bp_MissionLevel.CompleteMission` (`self.MissionLevel`) (`self.MissionIndex`))
  (`MovieSceneSequencePlayer.Play` _sequenceplayer))

(event `OnFinished`
  (`/Game/Gameplay/Core/bpc_MissionManager.ServerSelectMission` (`/Game/bfl_AccessHelper.GetMissionManager` self)))

(fn `UserConstructionScript`
  (bind _missionindex (`self.MissionIndex`))
  (`parent.UserConstructionScript`)
  (bind _returnvalue (`GameplayStatics.GetActorOfClass` "/Game/Gameplay/Missions/bp_MissionLevel.bp_MissionLevel_C"))
  (bind _output_get (set `self.MissionLevel` _returnvalue))
  (bind _missions (`/Game/Gameplay/Missions/bp_MissionLevel.Missions` _output_get))
  (if (`KismetArrayLibrary.Array_IsValidIndex` _missions _missionindex)
    (set `self.Mission` (`|GetArrayItem` _missions _missionindex))
    (else
      (set `self.Mission` (struct)))))