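; Respawn area actor that sets the respawn point for actors entering its trigger box.
; On the server, overlapping actors implementing Bpi_Respawn receive a world respawn point, computed from the root location plus the RespawnPoint offset.
; The construction script folds actor scale into BoxExtents, resets scale to one and resizes the trigger box, so scaling the actor resizes the volume.
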(event `self.SetRespawnTrigger.OnComponentBeginOverlap`
  (params (OverlappedComponent :type "PrimitiveComponent Object Reference") (OtherActor :type "Actor Object Reference") (OtherComp :type "PrimitiveComponent Object Reference") (OtherBodyIndex :type Integer) (bFromSweep :type Boolean) (SweepResult :type "HitResult Structure (by ref)"))
  (`/Engine/EditorBlueprintResources/ActorMacros.Switch Has Authority`
    (:`Authority`
      (if (`KismetSystemLibrary.DoesImplementInterface` OtherActor "/Game/Gameplay/Respawn/bpi_Respawn.bpi_Respawn_C")
        (message `/Game/Gameplay/Respawn/bpi_Respawn.SetRespawnPoint` OtherActor (`self.GetWorldRespawnPoint`))))))

(fn `GetWorldRespawnPoint`
  (returns (ReturnValue :type "Vector Structure"))
  (return (+ (`self.RespawnPoint`) (`SceneComponent.K2_GetComponentLocation` (`self.DefaultSceneRoot`)))))

(fn `UserConstructionScript`
  (bind _output_get (set `self.BoxExtents` (* (`self.GetActorScale3D`) (`self.BoxExtents`))))
  (`self.SetActorScale3D` (1.0 1.0 1.0))
  (`BoxComponent.SetBoxExtent` (`self.SetRespawnTrigger`) _output_get false))