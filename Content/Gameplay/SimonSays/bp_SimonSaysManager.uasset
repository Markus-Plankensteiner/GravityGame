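; Simon Says puzzle manager that shows a random color sequence for players to repeat on buttons.
; The construction script colors each composite and button pair and binds the buttons to the manager.
; On authority, a looping timer blinks the sequence, replaying it while no correct input has been made.
; Correct presses consume the sequence, ending in a green flash, disabled buttons and target trigger; mistakes flash red and reshuffle.
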(event `self.ReceiveBeginPlay`
  (`/Engine/EditorBlueprintResources/ActorMacros.Switch Has Authority`
    (:`Authority`
      (`self.RandomizeSequence` 5)
      (`self.StartBlink`))))

(event `BlinkNext`
  (bind (_output_color _output_composite) (break `/Game/Gameplay/SimonSays/s_SimonSaysSetup` (`|GetArrayItem` (`self.ColorSequence`) (`self.SequenceBlink`))))
  (`/Game/Gameplay/Props/Composite/bp_Composite.Trigger` _output_composite null)
  (if (< (`self.SequenceBlink`) (- (`KismetArrayLibrary.Array_Length` (`self.ColorSequence`)) 1))
    (`/Engine/EditorBlueprintResources/StandardMacros.IncrementInt` (`self.SequenceBlink`))
    (else
      (`self.StopBlink`)
      (`KismetSystemLibrary.Delay` 5.0)
      (if (== (`KismetArrayLibrary.Array_Length` (`self.ActiveSequence`)) (`KismetArrayLibrary.Array_Length` (`self.ColorSequence`)))
        (`self.StartBlink`)))))

(event `StartBlink`
  (set `self.SequenceBlink` 0)
  (bind _returnvalue (`KismetSystemLibrary.K2_SetTimerDelegate` (`|CreateDelegate` :!event `BlinkNext`) 2.0 true))
  (set `self.BlinkTimer` _returnvalue))

(event `StopBlink`
  (`KismetSystemLibrary.K2_ClearAndInvalidateTimerHandle` (`self.BlinkTimer`)))

(event `/Game/Gameplay/Props/Button/bpi_Trigger.Trigger`
  (params (Caller :type "Actor Object Reference"))
  (`self.IsCorrectInput` Caller
    (:`Yes`
      (`KismetSystemLibrary.PrintString` "Correct")
      (`KismetArrayLibrary.Array_Remove` (`self.ActiveSequence`))
      (if (`KismetArrayLibrary.Array_IsEmpty` (`self.ActiveSequence`))
        (`self.Full Blink` true)
        (`self.DeactivateButtons`)
        (if (`KismetSystemLibrary.DoesImplementInterface` (`self.TriggerTarget`) "/Game/Gameplay/Props/Button/bpi_Trigger.bpi_Trigger_C")
          (message `/Game/Gameplay/Props/Button/bpi_Trigger.Trigger` (`self.TriggerTarget`) self))))
    (:`No`
      (`self.Full Blink` false)
      (`self.RandomizeSequence` 5)
      (`KismetSystemLibrary.Delay` 2.0)
      (`self.StartBlink`))))

(fn `DeactivateButtons`
  (for _array_element (`self.ColorButtons`)
    (`/Game/Gameplay/Props/Button/bp_Button.SetActiveState` (`.Button_12_94D2C0A34F4624DED2A9A5A6A5CBA339` (break `/Game/Gameplay/SimonSays/s_SimonSaysSetup` _array_element)) false)))

(fn `Full Blink`
  (params (Success :type Boolean))
  (for _array_element (`self.ColorButtons`)
    (`/Game/Gameplay/Props/Composite/bp_Composite.MulticastTriggerColor` (`.Composite_11_F4425984468919185CE1B0BE30C6A52B` (break `/Game/Gameplay/SimonSays/s_SimonSaysSetup` _array_element)) (`KismetMathLibrary.SelectColor` (struct :`G` 1.0 :`A` 1.0) (struct :`R` 1.0 :`A` 1.0) Success)))
  (`self.StopBlink`))

(fn `RandomizeSequence`
  (params (SequenceLength :type Integer))
  (`KismetArrayLibrary.Array_Clear` (`self.ColorSequence`))
  (for _ (range 1 (+ SequenceLength 1))
    (`KismetArrayLibrary.Array_Add` (`self.ColorSequence`) (`KismetArrayLibrary.Array_Random` (`self.ColorButtons`))))
  (set `self.ActiveSequence` (`self.ColorSequence`))
  (return))

(fn `UserConstructionScript`
  (for _array_element (`self.ColorButtons`)
    (`|ExecutionSequence`
      (:`then_0`
        (`/Engine/EditorBlueprintResources/StandardMacros.IsValid` (`.Composite_11_F4425984468919185CE1B0BE30C6A52B` (break `/Game/Gameplay/SimonSays/s_SimonSaysSetup` _array_element))
          (:`Is Valid`
            (set `/Game/Gameplay/Props/Composite/bp_Composite.Color` (break `/Game/Gameplay/SimonSays/s_SimonSaysSetup` _array_element) (`.Composite_11_F4425984468919185CE1B0BE30C6A52B` (break `/Game/Gameplay/SimonSays/s_SimonSaysSetup` _array_element)))
            (`GravityGameFunctionLibrary.RerunConstructionScripts` (`.Composite_11_F4425984468919185CE1B0BE30C6A52B` (break `/Game/Gameplay/SimonSays/s_SimonSaysSetup` _array_element))))))
      (:`then_1`
        (`/Engine/EditorBlueprintResources/StandardMacros.IsValid` (`.Button_12_94D2C0A34F4624DED2A9A5A6A5CBA339` (break `/Game/Gameplay/SimonSays/s_SimonSaysSetup` _array_element))
          (:`Is Valid`
            (set `/Game/Gameplay/Props/Button/bp_Button.Color` (break `/Game/Gameplay/SimonSays/s_SimonSaysSetup` _array_element) (`.Button_12_94D2C0A34F4624DED2A9A5A6A5CBA339` (break `/Game/Gameplay/SimonSays/s_SimonSaysSetup` _array_element)))
            (set `/Game/Gameplay/Props/Button/bp_Button.Reset` true (`.Button_12_94D2C0A34F4624DED2A9A5A6A5CBA339` (break `/Game/Gameplay/SimonSays/s_SimonSaysSetup` _array_element)))
            (set `/Game/Gameplay/Props/Button/bp_Button.ResetTime` 0.3 (`.Button_12_94D2C0A34F4624DED2A9A5A6A5CBA339` (break `/Game/Gameplay/SimonSays/s_SimonSaysSetup` _array_element)))
            (set `/Game/Gameplay/Props/Button/bp_Button.Trigger` self (`.Button_12_94D2C0A34F4624DED2A9A5A6A5CBA339` (break `/Game/Gameplay/SimonSays/s_SimonSaysSetup` _array_element)))
            (`GravityGameFunctionLibrary.RerunConstructionScripts` (`.Button_12_94D2C0A34F4624DED2A9A5A6A5CBA339` (break `/Game/Gameplay/SimonSays/s_SimonSaysSetup` _array_element)))))))))