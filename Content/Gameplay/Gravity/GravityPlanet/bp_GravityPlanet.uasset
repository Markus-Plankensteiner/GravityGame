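; A planet actor that pulls an overlapping character's gravity toward its center.
; Sphere begin overlap caches the Bpc_GravityManager from the character's PlayerState and enables Tick, which submits the normalized direction from owner to planet at priority 0.
; The owner position comes from the manager's owner, the PlayerState, rather than the character directly.
; End overlap removes the gravity and disables Tick without checking which actor left; only one manager is tracked.
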(event `self.ReceiveTick`
  (params (DeltaSeconds :type "Float (single-precision)"))
  (`/Game/Gameplay/Gravity/bpc_GravityManager.SetGravity` (`self.PlayerGravityManager`) (make `/Game/Gameplay/Gravity/s_Gravity` self 0 (`KismetMathLibrary.Normal` (- (`self.K2_GetActorLocation`) (`self.K2_GetActorLocation` (`ActorComponent.GetOwner` (`self.PlayerGravityManager`))))))))

(event `self.Sphere.OnComponentBeginOverlap`
  (params (OverlappedComponent :type "PrimitiveComponent Object Reference") (OtherActor :type "Actor Object Reference") (OtherComp :type "PrimitiveComponent Object Reference") (OtherBodyIndex :type Integer) (bFromSweep :type Boolean) (SweepResult :type "HitResult Structure (by ref)"))
  (bind _ascharacter (cast `Character` OtherActor))
  (bind _returnvalue (`self.GetComponentByClass` (`Pawn.PlayerState` _ascharacter) "/Game/Gameplay/Gravity/bpc_GravityManager.bpc_GravityManager_C"))
  (`/Engine/EditorBlueprintResources/StandardMacros.IsValid` _returnvalue
    (:`Is Valid`
      (set `self.PlayerGravityManager` _returnvalue)
      (`self.SetActorTickEnabled` true))))

(event `self.Sphere.OnComponentEndOverlap`
  (params (OverlappedComponent :type "PrimitiveComponent Object Reference") (OtherActor :type "Actor Object Reference") (OtherComp :type "PrimitiveComponent Object Reference") (OtherBodyIndex :type Integer))
  (`/Game/Gameplay/Gravity/bpc_GravityManager.RemoveGravity` (`self.PlayerGravityManager`) self)
  (`self.SetActorTickEnabled` false))

(fn `UserConstructionScript`)