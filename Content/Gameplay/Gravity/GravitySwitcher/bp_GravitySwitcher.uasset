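; Gravity switcher volume that overrides the gravity of characters inside its GravityBounds.
; On overlap, it finds the Bpc_GravityManager component on the character's PlayerState and registers itself as a gravity source with its priority, speed and the forward vector of its GravityDirection component.
; On end overlap, it removes itself from that manager.
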(event `self.GravityBounds.OnComponentBeginOverlap`
  (params (OverlappedComponent :type "PrimitiveComponent Object Reference") (OtherActor :type "Actor Object Reference") (OtherComp :type "PrimitiveComponent Object Reference") (OtherBodyIndex :type Integer) (bFromSweep :type Boolean) (SweepResult :type "HitResult Structure (by ref)"))
  (bind _ascharacter (cast `Character` OtherActor))
  (bind _playerstate (`Pawn.PlayerState` _ascharacter)
    (:`then`
      (bind _returnvalue (`self.GetComponentByClass` _playerstate "/Game/Gameplay/Gravity/bpc_GravityManager.bpc_GravityManager_C"))
      (`/Engine/EditorBlueprintResources/StandardMacros.IsValid` _returnvalue
        (:`Is Valid`
          (`/Game/Gameplay/Gravity/bpc_GravityManager.SetGravity` _returnvalue (make `/Game/Gameplay/Gravity/s_Gravity` self (`self.Gravity Priority`) (`KismetMathLibrary.Conv_RotatorToVector` (`SceneComponent.K2_GetComponentRotation` (`self.GravityDirection`))) (`self.Gravity Speed`))))))
    (:`else`)))

(event `self.GravityBounds.OnComponentEndOverlap`
  (params (OverlappedComponent :type "PrimitiveComponent Object Reference") (OtherActor :type "Actor Object Reference") (OtherComp :type "PrimitiveComponent Object Reference") (OtherBodyIndex :type Integer))
  (bind _ascharacter (cast `Character` OtherActor))
  (bind _playerstate (`Pawn.PlayerState` _ascharacter)
    (:`then`
      (bind _returnvalue (`self.GetComponentByClass` _playerstate "/Game/Gameplay/Gravity/bpc_GravityManager.bpc_GravityManager_C"))
      (`/Engine/EditorBlueprintResources/StandardMacros.IsValid` _returnvalue
        (:`Is Valid`
          (`/Game/Gameplay/Gravity/bpc_GravityManager.RemoveGravity` _returnvalue self))))
    (:`else`)))

(fn `UserConstructionScript`)