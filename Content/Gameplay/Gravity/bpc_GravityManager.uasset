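; Gravity manager component on a PlayerState that steers the gravity direction of the player pawn's CharacterMovement.
; Gravity sources are added or removed by owner in a list, which the authority seeds on BeginPlay with a low-priority default.
; Each tick it moves current gravity at constant speed toward the highest-priority entry and applies it.
; The movement component is found through the pawn or set by a multicast event.
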(event `self.ReceiveBeginPlay`
  (`/Engine/EditorBlueprintResources/ActorComponentMacros.Switch Has Authority`
    (:`Authority`
      (`self.ResetGravity`))))

(event `self.ReceiveTick`
  (params (DeltaSeconds :type "Float (single-precision)"))
  (`self.CharacterMovement`
    (:`then`
      (bind _gravity (`/Game/Gameplay/Gravity/bpfl_Gravity.GetHighestPriorityGravity` (`self.TargetGravity`)))
      (bind _output_get (set `self.CurrentGravity` (`KismetMathLibrary.VInterpTo_Constant` (`self.CurrentGravity`) (`.Direction_10_C1689F3949BCDBD923BBFDA1C6FE056A` (break `/Game/Gameplay/Gravity/s_Gravity` _gravity)) DeltaSeconds (`.Speed_9_98D11FC04D5658A7B35EDDAF08EED7F1` (break `/Game/Gameplay/Gravity/s_Gravity` _gravity)))))
      (`CharacterMovementComponent.SetGravityDirection` (`self.CharacterMovement`) _output_get))
    (:`else`
      (bind _asplayer_state (cast `PlayerState` (`self.GetOwner`)))
      (bind _returnvalue (`PlayerState.GetPawn` _asplayer_state))
      (`/Engine/EditorBlueprintResources/StandardMacros.IsValid` _returnvalue
        (:`Is Valid`
          (set `self.CharacterMovement` (`Actor.GetComponentByClass` _returnvalue "/Script/Engine.CharacterMovementComponent")))))))

(event `MulticastSetCharacterMovement`
  (params (CharacterMovement :type "CharacterMovementComponent Object Reference"))
  (set `self.CharacterMovement` CharacterMovement))

(fn `RemoveGravity`
  (params (Owner :type "Actor Object Reference (by ref)"))
  (bind _gravityentries (`/Game/Gameplay/Gravity/bpfl_Gravity.GetGravityOfOwner` (`self.TargetGravity`) Owner))
  (for _array_element _gravityentries
    (`KismetArrayLibrary.Array_RemoveItem` (`self.TargetGravity`) _array_element)))

(fn `ResetGravity`
  (bind _targetgravity (`self.TargetGravity`))
  (`KismetArrayLibrary.Array_Clear` _targetgravity)
  (`KismetArrayLibrary.Array_Add` _targetgravity (make `/Game/Gameplay/Gravity/s_Gravity` null -999 (`self.DefaultGravity`))))

(fn `SetGravity`
  (params (Gravity :type "/Game/Gameplay/Gravity/s_Gravity Structure"))
  (`KismetArrayLibrary.Array_Add` (`self.TargetGravity`) Gravity))