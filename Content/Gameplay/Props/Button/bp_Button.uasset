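; Networked button prop that a ground-pounding bp_PlatformCharacter presses to send a Bpi_Trigger message to its linked Trigger actor.
; Overlap calls a server event, debounced by a resetting DoOnce, which sets or toggles the pressed state and can start a reset timer.
; Multicast timelines slide the mesh between Base sockets and drive color through custom primitive data.
; SetActiveState switches collision, presses the button and requests a grey fade.
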(event `self.ReceiveBeginPlay`
  (`/Engine/EditorBlueprintResources/ActorMacros.Switch Has Authority`
    (:`Authority`
      (set `self.OriginalPressed` (`self.Pressed`)))))

(event `self.Collision.OnComponentBeginOverlap`
  (params (OverlappedComponent :type "PrimitiveComponent Object Reference") (OtherActor :type "Actor Object Reference") (OtherComp :type "PrimitiveComponent Object Reference") (OtherBodyIndex :type Integer) (bFromSweep :type Boolean) (SweepResult :type "HitResult Structure (by ref)"))
  (`self.ServerButtonPressed` OtherActor))

(event `ServerButtonPressed`
  (params (Player :type "Actor Object Reference"))
  ;[1 1 1] Server Only
  (bind _asbp_platform_character (cast `/Game/Characters/bp_PlatformCharacter` Player))
  (if (`/Game/Characters/bp_PlatformCharacter.GroundPounding` _asbp_platform_character)
    (`|ExecutionSequence`
      (:`then_0`
        (`/Engine/EditorBlueprintResources/StandardMacros.DoOnce` false :!label _label
          (:`Completed`
            (if (`KismetSystemLibrary.DoesImplementInterface` (`self.Trigger`) "/Game/Gameplay/Props/Button/bpi_Trigger.bpi_Trigger_C")
              (message `/Game/Gameplay/Props/Button/bpi_Trigger.Trigger` (`self.Trigger`) self)
              (`self.SetPressedState` (select `bool` (`self.ToggleButton`) :`false` true :`true` (not (`self.Pressed`))))
              (else
                (`KismetSystemLibrary.PrintString` "ERROR: Button is not connected to a triggerable Actor" true true (struct :`R` 1.0 :`B` 0.025124 :`A` 1.0) 10.0))))))
      (:`then_1`
        (`KismetSystemLibrary.Delay` 0.2)
        (goto _label :!via `Reset`)))))

(event `DepressAfterDelay`
  ;[1 1 1] Server Only
  (if (`self.Active`)
    (`self.SetPressedState` (`self.OriginalPressed`))))

(event `MulticastFadeToColor`
  (params (Color :type "LinearColor Structure"))
  ;[1 1 1] Multicast / Client only
  (if (not (`KismetSystemLibrary.IsDedicatedServer`))
    (bind (_direction _fadelerp) (`Timeline|FadeColor` :!via `PlayFromStart`)
      (:`Update`
        (`self.SetColor` (`KismetMathLibrary.LinearColorLerp` (`self.Color`) Color _fadelerp))))))

(event `MulticastTriggerAnimation`
  (params (Forward :type Boolean))
  (bind _returnvalue (`SceneComponent.GetSocketLocation` (`self.Base`) "ButtonOut"))
  (bind _returnvalue_2 (`SceneComponent.GetSocketLocation` (`self.Base`) "ButtonIn"))
  ;[1 1 1] Multicast / Client only
  (bind (_direction _press) (`Timeline|Animation` :!via `PlayFromStart`)
    (:`Update`
      (`SceneComponent.K2_SetWorldLocation` (`self.Button`) (`KismetMathLibrary.VLerp` (`KismetMathLibrary.SelectVector` _returnvalue_2 _returnvalue Forward) (`KismetMathLibrary.SelectVector` _returnvalue _returnvalue_2 Forward) _press) false false))))

(fn `SetActiveState`
  (params (Active :type Boolean))
  (bind _output_get (set `self.Active` Active))
  (`PrimitiveComponent.SetCollisionEnabled` (`self.Collision`) (select `bool` _output_get :`false` "NoCollision" :`true` "QueryOnly" :!type "ECollisionEnabled Enum"))
  (`self.SetPressedState` true)
  (`self.MulticastFadeToColor` (struct :`R` 0.208333 :`G` 0.208333 :`B` 0.208333 :`A` 1.0)))

(fn `SetColor`
  (params (Color :type "LinearColor Structure"))
  (`PrimitiveComponent.SetDefaultCustomPrimitiveDataVector3` (`self.Button`) 0 (`KismetMathLibrary.MakeVector` Color_R Color_G Color_B)))

(fn `SetPressedState`
  (params (NewState :type Boolean))
  (if (!= NewState (`self.Pressed`))
    (bind _output_get (set `self.Pressed` NewState))
    (`self.MulticastTriggerAnimation` _output_get)
    (if (`self.Reset`)
      (bind _returnvalue (`KismetSystemLibrary.K2_SetTimerDelegate` (`|CreateDelegate` :!event `DepressAfterDelay`) (`self.ResetTime`)))
      (set `self.ResetTimer` _returnvalue))))

(fn `UserConstructionScript`
  (`SceneComponent.K2_SetWorldLocation` (`self.Button`) (select `bool` (`self.Pressed`) :`false` (`SceneComponent.GetSocketLocation` (`self.Base`) "ButtonOut") :`true` (`SceneComponent.GetSocketLocation` (`self.Base`) "ButtonIn")) false false)
  (if (not (`KismetSystemLibrary.IsDedicatedServer`))
    (`self.SetColor` (`self.Color`))))