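; Composite prop Blueprint whose static mesh blinks when triggered, in its own color or a temporary one.
; Trigger and color-trigger multicast events skip dedicated servers and restart a Blink timeline that feeds custom primitive data on the mesh.
; SetColor writes RGB as default custom primitive data, applied at construction, for color overrides, and to restore the configured color when the blink finishes.
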(event `/Game/Gameplay/Props/Button/bpi_Trigger.Trigger`
  (params (Caller :type "Actor Object Reference"))
  (`self.MulticastBlink`))

(event `MulticastBlink`
  (if (not (`KismetSystemLibrary.IsDedicatedServer`))
    (bind (_direction _blink) (`Timeline|Blink` :!via `PlayFromStart` :!label _label)
      (:`Update`
        (`PrimitiveComponent.SetCustomPrimitiveDataFloat` (`self.sm_Composite`) 0 _blink))
      (:`Finished`
        (`self.SetColor` (`self.Color`))))))

(event `MulticastTriggerColor`
  (params (BlinkColor :type "LinearColor Structure"))
  (if (not (`KismetSystemLibrary.IsDedicatedServer`))
    (`self.SetColor` BlinkColor)
    (goto _label :!via `PlayFromStart`)))

(fn `SetColor`
  (params (Color :type "LinearColor Structure"))
  (`PrimitiveComponent.SetDefaultCustomPrimitiveDataVector3` (`self.sm_Composite`) 1 (`KismetMathLibrary.MakeVector` Color_R Color_G Color_B)))

(fn `UserConstructionScript`
  (`self.SetColor` (`self.Color`)))