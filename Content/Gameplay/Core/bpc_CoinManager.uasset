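; Coin manager component that keeps a running count of collected coins.
; It exposes functions to read, increment and reset CoinCount.
; Collecting and resetting broadcast the new total through the OnCoinCountUpdated dispatcher.
; A RepNotify on CoinCount fires the same dispatcher, so listeners also hear about replicated changes.
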(fn `CollectedCoin`
  (bind _result (`/Engine/EditorBlueprintResources/StandardMacros.IncrementInt` (`self.CoinCount`))
    (:`  `
      (`self.OnCoinCountUpdated` _result))))

(fn `GetCoinCount`
  (returns (CoinCount :type Integer))
  (return (`self.CoinCount`)))

(fn `OnRep_CoinCount`
  (`self.OnCoinCountUpdated` (`self.CoinCount`)))

(fn `ResetCoins`
  (bind _output_get (set `self.CoinCount` 0))
  (`self.OnCoinCountUpdated` _output_get))