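; Mission manager component that moves players from the menu into gameplay when a mission is selected.
; It caches all PlayerStart actors on BeginPlay and stores the chosen mission when SelectedMission fires.
; It then spawns a Bp_Kazooie at the PlayerStart matching each PlayerController's index, has that controller possess it, and destroys every Bp_MenuCharacter.
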(event `self.ReceiveBeginPlay`
  (bind _outactors (`GameplayStatics.GetAllActorsOfClass` "/Script/Engine.PlayerStart"))
  (set `self.PlayerStarts` _outactors))

(event `Selected Mission`
  (params (Mission :type "/Game/Gameplay/Missions/s_Mission Structure"))
  (set `self.SelectedMission` Mission)
  (bind _outactors (`GameplayStatics.GetAllActorsOfClass` "/Script/Engine.PlayerController"))
  (for (_array_element _array_index) _outactors
    (bind (_returnvalue_location _returnvalue_rotation _returnvalue_scale) (`KismetMathLibrary.BreakTransform` (`Actor.GetTransform` (`|GetArrayItem` (`self.PlayerStarts`) _array_index))))
    (bind _returnvalue (`|SpawnActorFromClass` "/Game/Characters/Kazooie/bp_Kazooie.bp_Kazooie_C" (`KismetMathLibrary.MakeTransform` _returnvalue_location _returnvalue_rotation _returnvalue_scale) "AlwaysSpawn" "MultiplyWithRoot" null null))
    (`Controller.Possess` _array_element _returnvalue))
  (bind _outactors_2 (`GameplayStatics.GetAllActorsOfClass` "/Game/Characters/MenuPawn/bp_MenuCharacter.bp_MenuCharacter_C"))
  (for _array_element_2 _outactors_2
    (`Actor.K2_DestroyActor` _array_element_2)))